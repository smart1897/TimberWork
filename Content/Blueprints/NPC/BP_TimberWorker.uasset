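; BP_TimberWorker is an NPC woodcutter that plays axe-chopping animation and sound.
; It binds to its WoodComponent's cutting-wood event on BeginPlay, with a handler that starts or stops the axe attack montage from a boolean.
; When the AxeComponent begins overlapping an actor tagged "Wood", it plays the axe sound at the worker's location and plays the montage again.
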(event OnComponentBeginOverlap(AxeComponent)
  (params (OverlappedComponent :type Primitive%20Component%20Object%20Reference) (OtherActor :type Actor%20Object%20Reference) (OtherComp :type Primitive%20Component%20Object%20Reference) (OtherBodyIndex :type Integer) (bFromSweep :type Boolean) (SweepResult :type Hit%20Result%20Structure%20%28by%20ref%29))
  (if (Actor|ActorHasTag OtherActor "Wood")
    (Audio|PlaySoundatLocation "/Game/Assets/Sounds/Axe.Axe" (Transformation|GetActorLocation) "0, 0, 0" 1.0 1.0 0.0 0 0 0 0)
    (Animation|PlayAnimMontage "/Game/Assets/Characters/Mannequins/Animations/Manny/AxeAttackMontage.AxeAttackMontage" 1.0 "None")))

(event Custom|OnCuttingWoodEvent
  (params (Value :type Boolean))
  (if Value
    (Animation|PlayAnimMontage "/Game/Assets/Characters/Mannequins/Animations/Manny/AxeAttackMontage.AxeAttackMontage" 1.0 "None")
    (else
      (Animation|StopAnimMontage "/Game/Assets/Characters/Mannequins/Animations/Manny/AxeAttackMontage.AxeAttackMontage"))))

(event EventBeginPlay
  (EventDispatchers|BindEventtoOnCuttingWood (Variables|Default|GetWoodComponent) (EventDispatchers|CreateEvent :!event Custom|OnCuttingWoodEvent)))

(event Collision|EventActorBeginOverlap
  (params (OtherActor :type Actor%20Object%20Reference)))

(event EventTick
  (params (DeltaSeconds :type Float%20%28single-precision%29)))

(fn ConstructionScript)