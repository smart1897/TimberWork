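; BP_TimberSpectate is a spectator actor that can toggle a looping flight along a camera spline.
; On BeginPlay it caches the first BP_CamSpline found in the level.
; The IA_Spline input saves the current location and starts a timeline, scaled by Duration, that moves the actor along the spline without changing rotation.
; Pressing it again stops playback and restores the saved location.
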(event Custom|StartSpline
  (Components|Timeline|SetPlayRate (Variables|Default|GetTimeline) (/ 1.0 (Variables|Default|GetDuration)) :!label _label)
  (bind _newtrack_0 (Timeline|Timeline PlayFromStart)
    (:Update
      (Transformation|SetActorLocation (Spline|GetLocationatTime (Variables|/Game/Blueprints/Gameplay/BP_CamSpline.BP_CamSpline_C|GetSpline (Variables|Default|GetSplineRef)) _newtrack_0 "World" false) false false))
    (:Finished
      (goto _label))))

(event Input|EnhancedActionEvents|EnhancedInputActionIA_Spline
  (params (ActionValue :type Boolean) (ElapsedSeconds :type Float%20%28double-precision%29) (TriggeredSeconds :type Float%20%28double-precision%29) (InputAction :type Input%20Action%20Object%20Reference :default "/Game/Input/Actions/IA_Spline.IA_Spline"))
  (:Started
    (if (Audio|Components|Audio|IsPlaying (Variables|Default|GetTimeline))
      (Audio|Components|Audio|Stop (Variables|Default|GetTimeline))
      (Transformation|SetActorLocation (Variables|Default|GetLocation) false false)
      (else
        (Variables|Default|SetLocation (Transformation|GetActorLocation))
        (CallFunction|StartSpline)))))

(event EventBeginPlay
  (bind _outactors (Actor|GetAllActorsOfClass "/Game/Blueprints/Gameplay/BP_CamSpline.BP_CamSpline_C"))
  (if (> (Utilities|Array|Length _outactors) 0)
    (Variables|Default|SetSplineRef (Utilities|Array|Get(acopy) _outactors))))

(fn ConstructionScript)