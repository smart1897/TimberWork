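; Player camera manager that overrides BlueprintUpdateCamera to drive the view when the camera target is a timber worker.
; For targets tagged "Worker", it places the camera at the worker's FollowCamera location, using the player controller's rotation and default FOV.
; GetWorkerRef casts the target to BP_TimberWorker once and reuses that cached reference while it stays valid, even if the target changes.
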(event EventBeginPlay)

(event Collision|EventActorBeginOverlap
  (params (OtherActor :type Actor%20Object%20Reference)))

(event EventTick
  (params (DeltaSeconds :type Float%20%28single-precision%29)))

(fn ConstructionScript)

(fn BlueprintUpdateCamera
  (params (CameraTarget :type Actor%20Object%20Reference))
  (bind _workerref (CallFunction|GetWorkerRef CameraTarget))
  (if (Actor|ActorHasTag CameraTarget "Worker")
    (Utilities|IsValid _workerref
      (:Is%20Valid
        (return (Transformation|GetWorldLocation (Variables|/Script/TimberWork.TimberWorker|GetFollowCamera _workerref)) (Transformation|GetActorRotation (Game|GetPlayerController 0)) (Variables|Default|GetDefaultFOV) true)))))

(fn GetWorkerRef
  (params (Target :type Object%20Object%20Reference))
  (bind _workerref (Variables|Default|GetWorkerRef)
    (:then
      (return _workerref))
    (:else
      (bind _asbp_timber_worker (Utilities|Casting|CastToBP_TimberWorker Target))
      (bind _output_get (Variables|Default|SetWorkerRef _asbp_timber_worker))
      (return _output_get))))